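; BP_Zombie is an enemy pawn that chases pawns it sees and damages them on reaching them.
; PawnSensing drives AIMoveTo toward the seen pawn, applying damage on success or moving to a nearby random point on failure.
; TakeDamage updates health and Isdead, then unconditionally drops a MedKit, asks any valid Spawner for a new enemy, and destroys the zombie.
; Its bound OnTakeAnyDamage handler is empty.
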(event `OnTakeAnyDamage_Event` :!signature `self.OnTakeAnyDamage`
  (params (DamagedActor :type "Actor Object Reference") (Damage :type "Float (single-precision)") (DamageType :type "DamageType Object Reference") (InstigatedBy :type "Controller Object Reference") (DamageCauser :type "Actor Object Reference")))

(event `self.PawnSensing.OnSeePawn`
  (params (Pawn :type "Pawn Object Reference"))
  (`|AIMoveTo` self (0.0 0.0 0.0) Pawn 10.0
    (:`then`
      (add `self.OnTakeAnyDamage` (delegate `OnTakeAnyDamage_Event`)))
    (:`OnSuccess`
      (bind _output_get (set `self.DamageDone` 10.0))
      (`GameplayStatics.ApplyDamage` Pawn _output_get))
    (:`OnFail`
      (`|AIMoveTo` self (`NavigationSystemV1.K2_GetRandomReachablePointInRadius` (`self.K2_GetActorLocation`) 100.0 null null) null))))

(event `TakeDamage`
  (params (Damage :type "Float (double-precision)"))
  (bind _output_get (set `self.health` (- (`self.health`) Damage)))
  (set `self.isdead` (== _output_get 0.0))
  (`|SpawnActorFromClass` "/Game/Fab/MedKit.MedKit_C" (`self.GetTransform` self) "AdjustIfPossibleButAlwaysSpawn" "MultiplyWithRoot" null null)
  (bind _spawner (`self.Spawner`)
    (:`then`
      (`/Game/BP_Spawner.SpawnEnemy` _spawner))
    (:`else`
      _))
  (`self.K2_DestroyActor` self))

(fn `UserConstructionScript`)